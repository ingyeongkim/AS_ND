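; Main player controller that toggles between gameplay and a paused settings menu and hosts the spawn manager.
; On BeginPlay it adds the Enhanced Input mapping, enters game-only mode and spawns a SpawnManager at the origin.
; The mode-change action shows the settings UI through BP_MainHUD, switching to UI-only input with cursor and pause, while SetGameOnlyMode reverses this.
; NumPad 1 feeds the Easy data table row to the SpawnManager.
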(event Custom|SetGameOnlyMode
  (Input|SetInputModeGameOnly self false)
  (Variables|Default|SetbShowMouseCursor false)
  (Game|SetGamePaused false))

(event Custom|ShowSettingUI
  (bind _asbp_main_hud (Utilities|Casting|CastToBP_MainHUD (HUD|GetHUD)))
  (Default|ShowSettingUI _asbp_main_hud)
  (Input|SetInputModeUIOnly self 0 "DoNotLock" false)
  (Variables|Default|SetbShowMouseCursor true)
  (Game|SetGamePaused true))

(event Input|EnhancedActionEvents|EnhancedInputActionIA_ModeChange
  (params (ActionValue :type Boolean) (ElapsedSeconds :type Float%20%28double-precision%29) (TriggeredSeconds :type Float%20%28double-precision%29) (InputAction :type Input%20Action%20Object%20Reference :default "/Game/01_Blueprint/00_Global/Input/IA_ModeChange.IA_ModeChange"))
  (:Started
    (CallFunction|ShowSettingUI)))

(event EventBeginPlay
  (Input|AddMappingContext (PlayerController|LocalPlayerSubsystems|GetEnhancedInputLocalPlayerSubsystem self) "/Game/01_Blueprint/00_Global/Input/IM_PlayerControllerContext.IM_PlayerControllerContext" 0 "(bIgnoreAllPressedKeysUntilRelease=True,bForceImmediately=False,bNotifyUserSettings=False)")
  (CallFunction|SetGameOnlyMode)
  (bind _returnvalue (Game|SpawnActorfromClass "/Game/03_Data/Manager/SpawnManager.SpawnManager_C" (Math|Transform|MakeTransform "0, 0, 0") "Undefined" "MultiplyWithRoot" 0 0))
  (Variables|Default|SetSpawnManager _returnvalue))

(event EventTick
  (params (DeltaSeconds :type Float%20%28single-precision%29)))

(event Input|KeyboardEvents|NumPadOne
  (params (Key :type Key%20Structure :default "None"))
  (:Pressed
    (bind _returnvalue (Utilities|GetDataTableRow "/Game/03_Data/SpawnDataTable.SpawnDataTable" "Easy")
      (:then
        (Default|SpawnfromData (Variables|Default|GetSpawnManager) _returnvalue)))))

(fn ConstructionScript)