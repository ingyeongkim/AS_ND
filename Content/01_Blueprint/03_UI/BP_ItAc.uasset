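; BP_ItAc is a timed-interaction actor that destroys an assigned monster and itself once interaction is sustained long enough.
; SetMon assigns the monster, and Tick accumulates time while OnInteraction is set, resetting it otherwise.
; Tick feeds the remaining fraction to its InteractionUI widget through SetPer, then destroys both actors at MaxTime if the monster is valid.
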(event Custom|SetMon
  (params (MonsterActor :type Actor%20Object%20Reference))
  (bind _output_get (Variables|Default|SetMonsterActor MonsterActor)))

(event EventBeginPlay)

(event Collision|EventActorBeginOverlap
  (params (OtherActor :type Actor%20Object%20Reference)))

(event EventTick
  (params (DeltaSeconds :type Float%20%28single-precision%29))
  (bind _monsteractor (Variables|Default|GetMonsterActor))
  (if (Variables|Default|GetOnInteraction)
    (Variables|Default|SetAccTime (+ (Variables|Default|GetAccTime) DeltaSeconds))
    (else
      (Variables|Default|SetAccTime 0.0)))
  (bind _asinteraction_ui (Utilities|Casting|CastToInteractionUI (UserInterface|GetWidget (Variables|Default|GetWidget))))
  (Default|SetPer _asinteraction_ui (- 1.0 (/ (Variables|Default|GetAccTime) (Variables|Default|GetMaxTime))))
  (if (>= (Variables|Default|GetAccTime) (Variables|Default|GetMaxTime))
    (Utilities|IsValid _monsteractor
      (:Is%20Valid
        (Actor|DestroyActor _monsteractor)
        (Actor|DestroyActor)))))

(fn ConstructionScript)