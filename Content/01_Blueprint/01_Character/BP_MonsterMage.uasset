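; Player-controllable mage character with Enhanced Input movement, mana, projectile shots and an interaction-indicator actor it spawns and removes.
; AttackCheck sphere-traces forward, spawning a Niagara impact and a random-valued damage actor, and builds devil points shown on the HUD.
; An overhead-style widget component displays name, mana and devil count.
; Tick drives a material dissolve, and footstep traces read PM_Basic physical materials for effects, sounds and decals.
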(event Custom|AttackCheck
  (bind _returnvalue (Math|Random|RandomIntegerinRange 1 100))
  ;[1 1 1] 공격 체크
  (bind (_outhit _returnvalue_2) (Class|KismetSystemLibrary|SphereTraceSinglebyProfile (Transformation|GetActorLocation) (+ (Transformation|GetSocketLocation (Variables|Character|GetMesh) "None") (* (Transformation|GetActorForwardVector) 2e+02)) 0.0 "None" false 0 "ForDuration" true))
  (if _returnvalue_2
    (bind _returnvalue_3 (Niagara|SpawnSystematLocation "/Game/02_Resourse/Niagara/NA_AttackEffect.NA_AttackEffect" (.ImpactPoint (Collision|BreakHitResult _outhit)) (Transformation|GetActorRotation)))
    (Niagara|SetNiagaraVariable(Float) _returnvalue_3 "RandomSpritesizeMin" 3.0)
    (Niagara|SetNiagaraVariable(Float) _returnvalue_3 "RandomSpritesizeMax" 1e+01)
    (CallFunction|AddDevilPoint)
    (bind _returnvalue_4 (Game|SpawnActorfromClass "/Game/01_Blueprint/03_UI/DamageActor.DamageActor_C" (Math|Conversions|ToTransform(Vector) (.ImpactPoint (Collision|BreakHitResult _outhit))) "AlwaysSpawn" "MultiplyWithRoot" 0 0))
    (Default|InitDamageActor _returnvalue_4 _returnvalue (> _returnvalue 0))))

(event Custom|ManaUpdate
  ;[1 1 1] 마나 설정
  (bind _ascharacter_widget (Utilities|Casting|CastToCharacterWidget (UserInterface|GetWidget (Variables|Default|GetWidget))))
  (Default|SetPBPercent _ascharacter_widget (/ (Variables|StatusInfo|GetCurMana) (Variables|StatusInfo|GetMaxMana))))

(event Custom|SetCharacterName
  ;[1 1 1] 이름 설정
  (bind _ascharacter_widget (Utilities|Casting|CastToCharacterWidget (UserInterface|GetWidget (Variables|Default|GetWidget))))
  (Default|SetName _ascharacter_widget (Utilities|Text|ToText(Name) (.CharacterName (Utilities|Struct|BreakCharacterStructs (Variables|Ect|GetCharacterInfo))))))

(event Custom|Shooting_cc
  (bind _returnvalue (Transformation|GetActorTransform))
  ;[1 1 1] 프로젝타일 폰
  (Game|SpawnActorfromClass "/Game/01_Blueprint/02_Actor/BP_PlayerShootingBall.BP_PlayerShootingBall_C" (Math|Transform|MakeTransform (+ (Transformation|GetActorLocation) (* (Transformation|GetActorForwardVector) 1.3e+02)) (.rotation _returnvalue) (.scale _returnvalue)) "Undefined" "MultiplyWithRoot" 0 0))

(event Custom|FootStep
  (params (IsLeft :type Boolean))
  ;[1 1 1] 발걸음 효과
  (CallFunction|FuncFootstep IsLeft))

(event Custom|InterectionUIOn
  (params (NPCLoca :type Vector) (Mon :type Actor%20Object%20Reference))
  (bind _returnvalue (Game|SpawnActorfromClass "/Game/01_Blueprint/03_UI/BP_ItAc.BP_ItAc_C" (Math|Conversions|ToTransform(Vector) NPCLoca) "Undefined" "MultiplyWithRoot" 0 0))
  (bind _output_get (Variables|Ect|SetInterectionActor _returnvalue))
  (Default|SetMon _output_get Mon))

(event Custom|InterectionUIOff
  (Utilities|IsValid (Variables|Ect|GetInterectionActor)
    (:Is%20Valid
      (Actor|DestroyActor (Variables|Ect|GetInterectionActor))
      (Variables|Ect|SetInterectionActor 0))))

(event Input|EnhancedActionEvents|EnhancedInputActionIA_MouseXY
  (params (ActionValue :type Vector%202D%20Structure) (ElapsedSeconds :type Float%20%28double-precision%29) (TriggeredSeconds :type Float%20%28double-precision%29) (InputAction :type Input%20Action%20Object%20Reference :default "/Game/01_Blueprint/00_Global/Input/IA_MouseXY.IA_MouseXY"))
  ;[1 1 1] 키보드 마우스 입력 처리
  (Pawn|Input|AddControllerYawInput (.x ActionValue))
  (Pawn|Input|AddControllerPitchInput (.y ActionValue)))

(event Input|EnhancedActionEvents|EnhancedInputActionIA_Jump
  (params (ActionValue :type Boolean) (ElapsedSeconds :type Float%20%28double-precision%29) (TriggeredSeconds :type Float%20%28double-precision%29) (InputAction :type Input%20Action%20Object%20Reference :default "/Game/01_Blueprint/00_Global/Input/IA_Jump.IA_Jump"))
  ;[1 1 1] 키보드 마우스 입력 처리
  (Character|Jump))

(event Input|EnhancedActionEvents|EnhancedInputActionIA_MoveForward
  (params (ActionValue :type Float%20%28double-precision%29) (ElapsedSeconds :type Float%20%28double-precision%29) (TriggeredSeconds :type Float%20%28double-precision%29) (InputAction :type Input%20Action%20Object%20Reference :default "/Game/01_Blueprint/00_Global/Input/IA_MoveForward.IA_MoveForward"))
  ;[1 1 1] 키보드 마우스 입력 처리
  (Pawn|Input|AddMovementInput (Math|Vector|GetForwardVector (Math|Rotator|MakeRotator 0.0 0.0 (.yaw (Pawn|GetControlRotation :!class /Script/Engine.Pawn)))) ActionValue false))

(event Input|EnhancedActionEvents|EnhancedInputActionIA_MoveRight
  (params (ActionValue :type Float%20%28double-precision%29) (ElapsedSeconds :type Float%20%28double-precision%29) (TriggeredSeconds :type Float%20%28double-precision%29) (InputAction :type Input%20Action%20Object%20Reference :default "/Game/01_Blueprint/00_Global/Input/IA_MoveRight.IA_MoveRight"))
  ;[1 1 1] 키보드 마우스 입력 처리
  (Pawn|Input|AddMovementInput (Math|Vector|GetForwardVector (Math|Rotator|MakeRotator 0.0 0.0 (.yaw (Pawn|GetControlRotation :!class /Script/Engine.Pawn)))) ActionValue false))

(event EventBeginPlay
  ;[1 1 1] 매핑 컨텍스트 세팅
  (Utilities|FlowControl|Sequence
    (:then_0
      (bind _as플레이어_컨트롤러 (Utilities|Casting|CastToPlayerController (Pawn|GetController)))
      (Utilities|IsValid _as플레이어_컨트롤러
        (:Is%20Valid
          (Input|AddMappingContext (PlayerController|LocalPlayerSubsystems|GetEnhancedInputLocalPlayerSubsystem _as플레이어_컨트롤러) "/Game/01_Blueprint/00_Global/Input/IM_Context.IM_Context" 0 "(bIgnoreAllPressedKeysUntilRelease=True,bForceImmediately=False,bNotifyUserSettings=False)"))))
    (:then_1
      (CallFunction|ManaUpdate)
      (CallFunction|SetCharacterName))
    (:then_2
      (for _index (range 0 0)
        _))))

(event EventTick
  (params (DeltaSeconds :type Float%20%28single-precision%29))
  (Utilities|FlowControl|Sequence
    (:then_0
      ;[1 1 1] 디졸브 처리
      (CallFunction|Dissolve DeltaSeconds))))

(fn ConstructionScript)

(fn AddDevilPoint
  ;[1 1 1] 데빌 포인트 쌓기
  (bind _result (Math|Integer|IncrementInt (Variables|StatusInfo|GetCurDevilPoint))
    (:%20%20
      (if (> _result (Variables|StatusInfo|GetMaxDevilPoint))
        (Variables|StatusInfo|SetCurDevilPoint (Variables|StatusInfo|GetMaxDevilPoint)))
      ;[1 1 1] 데빌 포인트가 가득 차면 플레이어 위젯에 악마 추가
      (if (== (Variables|StatusInfo|GetMaxDevilPoint) (Variables|StatusInfo|GetCurDevilPoint))
        (if (> (+ (Variables|StatusInfo|GetCompliteDevil) 1) (Variables|StatusInfo|GetMaxCompliteDevil))
          _
          (else
            (Variables|StatusInfo|SetCompliteDevil 0)
            (Variables|StatusInfo|SetCurDevilPoint 0))))
      ;[1 1 1] MainUI에 데빌 포인트를 퍼센트 단위로 쌓음
      (bind _asbp_main_hud (Utilities|Casting|CastToBP_MainHUD (HUD|GetHUD (Game|GetPlayerController 0))))
      (Default|SetDevilPointPercent (Variables|/Game/01_Blueprint/03_UI/BP_MainHUD.BP_MainHUD_C|GetMainUI _asbp_main_hud) (/ (Variables|StatusInfo|GetCurDevilPoint) (Variables|StatusInfo|GetMaxDevilPoint)))
      (Development|PrintString (Utilities|String|ToString(Float) (/ (Variables|StatusInfo|GetCurDevilPoint) (Variables|StatusInfo|GetMaxDevilPoint))))
      (bind _ascharacter_widget (Utilities|Casting|CastToCharacterWidget (UserInterface|GetWidget (Variables|Default|GetWidget))))
      (Default|SetDevilPoint _ascharacter_widget (Variables|StatusInfo|GetCompliteDevil) (Variables|StatusInfo|GetMaxCompliteDevil)))))

(fn Shooting
  (bind _returnvalue (Transformation|GetActorTransform))
  (Game|SpawnActorfromClass "/Game/01_Blueprint/01_Character/BP_Bullet.BP_Bullet_C" (Math|Transform|MakeTransform (+ (.location _returnvalue) (* (Transformation|GetActorForwardVector) 8e+01)) (.rotation _returnvalue) (.scale _returnvalue)) "Undefined" "MultiplyWithRoot" 0 0)
  (bind _asbp_main_game_mode (Utilities|Casting|CastToBP_MainGameMode (Game|GetGameMode)))
  (Default|CheckGameModeCandoti _asbp_main_game_mode))

(fn Dissolve
  (params (DeltaSecond :type Float%20%28double-precision%29))
  (if (Variables|Ect|GetDissolveOn)
    (if (> (Variables|Ect|GetDissolveTime) -1.0)
      (bind _output_get (Variables|Ect|SetDissolveTime (- (Variables|Ect|GetDissolveTime) DeltaSecond)))
      (Rendering|Material|SetScalarParameterValueonMaterials (Variables|Character|GetMesh) "None" _output_get))
    (elif (< (Variables|Ect|GetDissolveTime) 2.0)
      (Variables|Ect|SetDissolveTime (+ (Variables|Ect|GetDissolveTime) DeltaSecond))
      (Rendering|Material|SetScalarParameterValueonMaterials (Variables|Character|GetMesh) "None" (Variables|Ect|GetDissolveTime)))))

(fn FuncFootstep
  (params (IsLeft :type Boolean))
  (bind _mesh (Variables|Character|GetMesh))
  (bind _returnvalue (Transformation|GetWorldRotation _mesh))
  (if true
    (Variables|Ect|SetFootLocation (Transformation|GetSocketLocation (Variables|Collision|GetCapsuleComponent) "None"))
    (else
      (Variables|Ect|SetFootLocation (Transformation|GetSocketLocation (Variables|Collision|GetCapsuleComponent) "None"))))
  (bind (_outhit _returnvalue_2) (Collision|LineTraceByChannel (Variables|Ect|GetFootLocation) (+ (Variables|Ect|GetFootLocation) "") "TraceTypeQuery1" false 0 "None"))
  (if _returnvalue_2
    (bind _aspm_basic (Utilities|Casting|CastToPM_Basic (.PhysMat (Collision|BreakHitResult _outhit)))
      (:then
        (Niagara|SpawnSystematLocation (Variables|/Game/02_Resourse/Material/PM_Basic.PM_Basic_C|GetNaFootWalk _aspm_basic) (.ImpactPoint (Collision|BreakHitResult _outhit)) _returnvalue)
        (Audio|PlaySoundatLocation (Variables|/Game/02_Resourse/Material/PM_Basic.PM_Basic_C|GetFootSound _aspm_basic) (.ImpactPoint (Collision|BreakHitResult _outhit)) "0, 0, 0" 1.0 1.0 0.0 0 0 0 0)
        (Game|SpawnActorfromClass (Variables|/Game/02_Resourse/Material/PM_Basic.PM_Basic_C|GetDecal _aspm_basic) (Math|Transform|MakeTransform (.ImpactPoint (Collision|BreakHitResult _outhit)) _returnvalue "1.000000,1.000000,1.000000") "AlwaysSpawn" "MultiplyWithRoot" 0 0))
      (:CastFailed
        (Development|PrintString "Hello")))
    (else
      (Development|PrintString "Hello"))))

(fn AttackSpentMana
  (if (>= (- (Variables|StatusInfo|GetCurMana) (Variables|StatusInfo|GetSpentMana)) 0.0)
    (Variables|StatusInfo|SetCurMana (- (Variables|StatusInfo|GetCurMana) (Variables|StatusInfo|GetSpentMana))))
  (CallFunction|ManaUpdate)
  (return (>= (- (Variables|StatusInfo|GetCurMana) (Variables|StatusInfo|GetSpentMana)) 0.0)))