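; BP_UpgradeCube3 is a moving cube actor whose static mesh shuttles back and forth between its starting relative location and a target component's location.
; BeginPlay caches both endpoints, and Tick moves the mesh along the normalized direction at Speed scaled by delta time, without sweep.
; When the travelled distance reaches the segment length, start and target swap through a temporary variable, reversing the motion.
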(event EventBeginPlay
  (Variables|Default|SetStartLocation (Variables|/Script/Engine.SceneComponent|GetRelativeLocation (Variables|Default|GetStaticMesh)))
  (Variables|Default|SetTargetLocation (Variables|/Script/Engine.SceneComponent|GetRelativeLocation (Variables|Default|GetTartgetComponent))))

(event Collision|EventActorBeginOverlap
  (params (OtherActor :type Actor%20Object%20Reference)))

(event EventTick
  (params (DeltaSeconds :type Float%20%28single-precision%29))
  (Utilities|FlowControl|Sequence
    (:then_0
      ;[1 1 1] 가야할 거리
      (Variables|Default|SetLength (Math|Vector|VectorLength (- (Variables|Default|GetTargetLocation) (Variables|Default|GetStartLocation)))))
    (:then_1
      ;[1 1 1] 가고 있는 거리
      (Variables|Default|SetTravelled (Math|Vector|VectorLength (- (Variables|/Script/Engine.SceneComponent|GetRelativeLocation (Variables|Default|GetStaticMesh)) (Variables|Default|GetStartLocation)))))
    (:then_2
      ;[1 1 1] 위치 셔플 바꾸기
      (if (>= (Variables|Default|GetTravelled) (Variables|Default|GetLength))
        (Variables|Default|SetTempLocation (Variables|Default|GetStartLocation))
        (Variables|Default|SetStartLocation (Variables|Default|GetTargetLocation))
        (Variables|Default|SetTargetLocation (Variables|Default|GetTempLocation))))
    (:then_3
      ;[1 1 1] 이동
      (Transformation|SetRelativeLocation (Variables|Default|GetStaticMesh) (+ (Variables|/Script/Engine.SceneComponent|GetRelativeLocation (Variables|Default|GetStaticMesh)) (* (Math|Vector|Normalize (- (Variables|Default|GetTargetLocation) (Variables|Default|GetStartLocation))) (* (Variables|Default|GetSpeed) DeltaSeconds))) false false))))

(fn ConstructionScript)