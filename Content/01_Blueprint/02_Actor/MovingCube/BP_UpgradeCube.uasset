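; BP_UpgradeCube is a moving cube actor that shuttles its static mesh back and forth between its starting position and a target component's position.
; Each Tick compares distance travelled to path length, then moves the mesh along the normalized direction at Speed in relative space, without sweep.
; On arrival, Shuffle swaps start and target and sets IsWait, pausing movement for three seconds before the return trip.
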(event EventBeginPlay
  (Variables|Default|SetStartLocation (Variables|/Script/Engine.SceneComponent|GetRelativeLocation (Variables|Default|GetStaticMesh)))
  (Variables|Default|SetTargetLocation (Variables|/Script/Engine.SceneComponent|GetRelativeLocation (Variables|Default|GetTartgetComponent))))

(event Collision|EventActorBeginOverlap
  (params (OtherActor :type Actor%20Object%20Reference)))

(event EventTick
  (params (DeltaSeconds :type Float%20%28single-precision%29))
  (if (Variables|Default|GetIsWait)
    (CallFunction|WaitTimeCheck DeltaSeconds)
    (else
      (CallFunction|LengthCheck)
      (bind _ischange (CallFunction|Shuffle))
      (Variables|Default|SetIsWait _ischange)
      (CallFunction|MoveUpdate DeltaSeconds))))

(fn ConstructionScript)

(fn MoveUpdate
  (params (DeltaTime :type Float%20%28double-precision%29))
  ;[1 1 1] 이동
  (Transformation|SetRelativeLocation (Variables|Default|GetStaticMesh) (+ (Variables|/Script/Engine.SceneComponent|GetRelativeLocation (Variables|Default|GetStaticMesh)) (* (Math|Vector|Normalize (- (Variables|Default|GetTargetLocation) (Variables|Default|GetStartLocation))) (* (Variables|Default|GetSpeed) DeltaTime))) false false))

(fn LengthCheck
  ;[1 1 1] 가야할 거리
  (Variables|Default|SetLength (Math|Vector|VectorLength (- (Variables|Default|GetTargetLocation) (Variables|Default|GetStartLocation))))
  ;[1 1 1] 가고 있는 거리
  (Variables|Default|SetTravelled (Math|Vector|VectorLength (- (Variables|/Script/Engine.SceneComponent|GetRelativeLocation (Variables|Default|GetStaticMesh)) (Variables|Default|GetStartLocation)))))

(fn Shuffle
  (bind _length (Variables|Default|GetLength))
  (bind _travelled (Variables|Default|GetTravelled))
  (bind _returnvalue (>= _travelled _length))
  ;[1 1 1] 위치 셔플 바꾸기
  (if _returnvalue
    (Variables|Default|SetTempLocation (Variables|Default|GetStartLocation))
    (Variables|Default|SetStartLocation (Variables|Default|GetTargetLocation))
    (Variables|Default|SetTargetLocation (Variables|Default|GetTempLocation))
    (return _returnvalue)
    (else
      (return false))))

(fn WaitTimeCheck
  (params (DeltaTime :type Float%20%28double-precision%29))
  (bind _output_get (Variables|Default|SetAccTime (+ (Variables|Default|GetAccTime) DeltaTime)))
  (if (>= _output_get 3.0)
    (Variables|Default|SetIsWait false)
    (Variables|Default|SetAccTime 0.0)))