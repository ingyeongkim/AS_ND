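; A moving cube actor that shuttles its mesh between its starting position and a target component's position, with a projectile-firing function.
; Tick moves it at Speed, swapping endpoints on arrival; when IsWait is set, it only runs a wait timer that never clears the flag.
; Shooting spawns BP_ChoiceCubeBullet ahead of the mesh but is never called here, and the cooldown timer adds zero each tick.
; Despite the Rotate name, no rotation logic is present.
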(event EventBeginPlay
  (Variables|Default|SetStartLocation (Variables|/Script/Engine.SceneComponent|GetRelativeLocation (Variables|Default|GetStaticMesh)))
  (Variables|Default|SetTargetLocation (Variables|/Script/Engine.SceneComponent|GetRelativeLocation (Variables|Default|GetTartgetComponent))))

(event Collision|EventActorBeginOverlap
  (params (OtherActor :type Actor%20Object%20Reference)))

(event EventTick
  (params (DeltaSeconds :type Float%20%28single-precision%29))
  (Utilities|FlowControl|Sequence
    (:then_0
      (if (Variables|Default|GetIsWait)
        (CallFunction|WaitMove DeltaSeconds)
        (else
          (CallFunction|DontStopMove DeltaSeconds))))
    (:then_1
      (CallFunction|ComputeShootingTime))))

(fn ConstructionScript)

(fn MoveUpdate
  (params (DeltaTime :type Float%20%28double-precision%29))
  ;[1 1 1] 이동
  (Transformation|SetRelativeLocation (Variables|Default|GetStaticMesh) (+ (Variables|/Script/Engine.SceneComponent|GetRelativeLocation (Variables|Default|GetStaticMesh)) (* (Math|Vector|Normalize (- (Variables|Default|GetTargetLocation) (Variables|Default|GetStartLocation))) (* (Variables|Default|GetSpeed) DeltaTime))) false false))

(fn LengthCheck
  ;[1 1 1] 가야할 거리
  (Variables|Default|SetLength (Math|Vector|VectorLength (- (Variables|Default|GetTargetLocation) (Variables|Default|GetStartLocation))))
  ;[1 1 1] 가고 있는 거리
  (Variables|Default|SetTravelled (Math|Vector|VectorLength (- (Variables|/Script/Engine.SceneComponent|GetRelativeLocation (Variables|Default|GetStaticMesh)) (Variables|Default|GetStartLocation)))))

(fn Shuffle
  (bind _length (Variables|Default|GetLength))
  (bind _travelled (Variables|Default|GetTravelled))
  (bind _returnvalue (>= _travelled _length))
  ;[1 1 1] 위치 셔플 바꾸기
  (if _returnvalue
    (Variables|Default|SetTempLocation (Variables|Default|GetStartLocation))
    (Variables|Default|SetStartLocation (Variables|Default|GetTargetLocation))
    (Variables|Default|SetTargetLocation (Variables|Default|GetTempLocation))
    (return _returnvalue)
    (else
      (return false))))

(fn WaitTimeCheck
  (params (DeltaTime :type Float%20%28double-precision%29))
  (bind _output_get (Variables|Default|SetAccTime (+ (Variables|Default|GetAccTime) DeltaTime)))
  (if (>= _output_get 3.0)
    (Variables|Default|SetIsWait true)
    (Variables|Default|SetAccTime 0.0)))

(fn DontStopMove
  (params (DeltaTime :type Float%20%28double-precision%29))
  (CallFunction|LengthCheck)
  (CallFunction|Shuffle)
  (CallFunction|MoveUpdate DeltaTime))

(fn WaitMove
  (params (DeltaTime :type Float%20%28double-precision%29))
  (if (Variables|Default|GetIsWait)
    (CallFunction|WaitTimeCheck DeltaTime)
    (else
      (CallFunction|LengthCheck)
      (bind _ischange (CallFunction|Shuffle))
      (Variables|Default|SetIsWait _ischange)
      (CallFunction|MoveUpdate 0.0))))

(fn ComputeShootingTime
  (bind _output_get (Variables|Default|SetProjecttileAccTime (+ (Variables|Default|GetProjecttileAccTime) 0.0)))
  (if (>= _output_get (Variables|Default|GetProjecttileShootingCoolTime))
    (Variables|Default|SetProjecttileAccTime 0.0)))

(fn Shooting
  (bind _staticmesh (Variables|Default|GetStaticMesh))
  (bind _returnvalue (Transformation|GetWorldTransform _staticmesh))
  (Game|SpawnActorfromClass "/Game/01_Blueprint/02_Actor/MovingCube/BP_ChoiceCubeBullet.BP_ChoiceCubeBullet_C" (Math|Transform|MakeTransform (+ (.location _returnvalue) (* (Transformation|GetActorForwardVector) 8e+01)) (.rotation _returnvalue) (.scale _returnvalue)) "Undefined" "MultiplyWithRoot" 0 0))