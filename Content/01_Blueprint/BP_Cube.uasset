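; BP_Cube is an actor that shuttles back and forth along a configurable direction vector.
; Each Tick it accumulates elapsed time and moves by the normalized Dir times Speed and delta time, forward or reversed depending on the Go flag.
; Once the timer passes three seconds, it flips Go, resets the timer and prints the new state.
; An unconnected leftover branch holds an earlier absolute-position movement attempt.
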(event EventBeginPlay)

(event Collision|EventActorBeginOverlap
  (params (OtherActor :type Actor%20Object%20Reference)))

(event EventTick
  (params (DeltaSeconds :type Float%20%28single-precision%29))
  (Utilities|FlowControl|Sequence
    (:then_0
      ;[1 1 1] AccTime 더하기
      (Variables|Default|SetAccTime (+ (Variables|Default|GetAccTime) DeltaSeconds)))
    (:then_1
      ;[1 1 1] Go bool 값에 따른 움직임
      (if (Variables|Default|GetGo)
        ;[1 1 1] 올라가기
        (Transformation|SetActorLocation (+ (Transformation|GetActorLocation) (* (* (Math|Vector|Normalize (Variables|Default|GetDir)) (Variables|Default|GetSpeed)) DeltaSeconds)) false false)
        (else
          ;[1 1 1] 내려가기
          (Transformation|SetActorLocation (+ (Transformation|GetActorLocation) (* (* (Math|Vector|Normalize (* (Variables|Default|GetDir) -1.0)) (Variables|Default|GetSpeed)) DeltaSeconds)) false false))))
    (:then_2
      ;[1 1 1] Go bool값 세팅하기
      (if (> (Variables|Default|GetAccTime) 3.0)
        (if (Variables|Default|GetGo)
          (Variables|Default|SetGo false)
          (else
            (Variables|Default|SetGo true)))
        (Variables|Default|SetAccTime 0.0)
        (Development|PrintString (Utilities|String|ToString(Boolean) (Variables|Default|GetGo)))))))

(fn ConstructionScript)